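; Pullable lever for a code console that reports its pull value to listeners when it reaches the down position.
; A pull plays a sound, stops the mesh blocking a custom trace channel and drives its roll rotation with a timeline.
; When the forward motion finishes, it fires the lever-down dispatcher, then resets after a delay.
; Reset restores blocking as the timeline starts reversing, before the lever is fully back up.
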(event `Event_Pull`
  (`GameplayStatics.PlaySoundAtLocation` null (`self.K2_GetActorLocation` self) (struct) 1.0 1.0 0.0 null null null null)
  (`PrimitiveComponent.SetCollisionResponseToChannel` (`self.StaticMesh`) "ECC_GameTraceChannel2" "ECR_Ignore")
  (bind (_direction _movement) (`Timeline|Timeline` :`NewTime` 2.0 :!label _label)
    (:`Update`
      (`SceneComponent.K2_SetRelativeRotation` (`self.StaticMesh`) (`KismetMathLibrary.MakeRotator` _movement) false false))
    (:`Finished`
      (switch `ETimelineDirection` _direction
        (:`Forward`
          (`self.OnLeverDown` self (`self.PullValue`))
          (`KismetSystemLibrary.Delay` 5.0)
          (`self.Event_Reset`))))))

(event `Event_Reset`
  (`PrimitiveComponent.SetCollisionResponseToChannel` (`self.StaticMesh`) "ECC_GameTraceChannel2" "ECR_Block")
  (goto _label :!via `Reverse`))

(fn `UserConstructionScript`)