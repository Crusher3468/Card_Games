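; Number wheel for a slot-style code console that spins and stops on a random digit position from 0 to 9.
; Event_RotateTo plays the spin audio and runs a looping timer that steps the mesh's roll through Event_Spin.
; After a fixed delay, it snaps to a hard-coded digit angle, stops the audio and plays a sound.
; Value and the angle come from separate random evaluations, so they can differ.
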(event `Event_RotateTo`
  (bind _returnvalue (`KismetMathLibrary.RandomIntegerInRange` 0 9))
  (`AudioComponent.Play` (`self.Spin`) 0.0)
  (set `self.Value` _returnvalue)
  (switch `int` _returnvalue
    (:`0`
      (set `self.DesiredRotation` 30.0))
    (:`1`
      (set `self.DesiredRotation` -10.0))
    (:`2`
      (set `self.DesiredRotation` -40.0))
    (:`3`
      (set `self.DesiredRotation` -80.0))
    (:`4`
      (set `self.DesiredRotation` -110.0))
    (:`5`
      (set `self.DesiredRotation` -150.0))
    (:`6`
      (set `self.DesiredRotation` 170.0))
    (:`7`
      (set `self.DesiredRotation` 140.0))
    (:`8`
      (set `self.DesiredRotation` 100.0))
    (:`9`
      (set `self.DesiredRotation` 60.0)))
  (bind _returnvalue_2 (`KismetSystemLibrary.K2_SetTimerDelegate` (delegate `Event_Spin`) 0.05 true))
  (`KismetSystemLibrary.Delay` 4.0)
  (`KismetSystemLibrary.K2_ClearAndInvalidateTimerHandle` _returnvalue_2)
  (`SceneComponent.K2_SetRelativeRotation` (`self.StaticMesh`) (`KismetMathLibrary.MakeRotator` (`self.DesiredRotation`)) false false)
  (`AudioComponent.Stop` (`self.Spin`))
  (`GameplayStatics.PlaySoundAtLocation` null (`self.K2_GetActorLocation` self) (struct) 1.0 1.0 0.0 null null null null))

(event `Event_Spin`
  (`SceneComponent.K2_AddRelativeRotation` (`self.StaticMesh`) (struct :`Roll` 10.0) false false))

(fn `UserConstructionScript`)