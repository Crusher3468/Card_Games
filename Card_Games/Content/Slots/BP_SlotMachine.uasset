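; Slot machine actor that spins its reels when the child lever actor is pulled and pays out money by matching card suits.
; BeginPlay binds the lever event, shows the W_Slots widget and switches to UI-only mouse input.
; RollSlots rotates each spinner, then maps its 0–9 value to an unevenly weighted suit.
; Count tallies the suits, and pairs, triples or four-of-a-kinds add rewards directly to the widget's Money.
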(event `self.ReceiveBeginPlay`
  (bind _returnvalue (`GameplayStatics.GetPlayerController` 0))
  (bind _asbp_code_console_lever (cast `/Game/Slots/BP_CodeConsole_Lever` (`ChildActorComponent.ChildActor` (`self.Lever`))))
  (add `/Game/Slots/BP_CodeConsole_Lever.OnLeverDown` _asbp_code_console_lever (delegate `RollSlots`))
  (bind _returnvalue_2 (`|CreateWidget` "/Game/Slots/W_Slots.W_Slots_C"))
  (bind _output_get (set `self.Widget` _returnvalue_2))
  (`UserWidget.AddToViewport` _output_get 0)
  (`WidgetBlueprintLibrary.SetInputMode_UIOnlyEx` _returnvalue null "LockAlways")
  (set `PlayerController.bShowMouseCursor` true _returnvalue))

(event `RollSlots`
  (params (Lever :type "/Game/Slots/BP_CodeConsole_Lever Object Reference") (Value :type Integer))
  (bind _widget (`self.Widget`))
  (bind _widget_2 (`self.Widget`))
  (bind _widget_3 (`self.Widget`))
  (bind _widget_4 (`self.Widget`))
  (bind _spinners (`self.Spinners`))
  (bind _widget_5 (`self.Widget`))
  (bind _widget_6 (`self.Widget`))
  (bind _widget_7 (`self.Widget`))
  (bind _widget_8 (`self.Widget`))
  (bind _widget_9 (`self.Widget`))
  (bind _widget_10 (`self.Widget`))
  (bind _widget_11 (`self.Widget`))
  (bind _widget_12 (`self.Widget`))
  (`KismetArrayLibrary.Array_Clear` (`self.Suits`))
  (for _array_element _spinners
    (`/Game/Slots/BP_CodeConsole_NumberWheel.Event_RotateTo` _array_element))
  (for _array_element_2 _spinners
    (bind _output_get (set `self.Value` (`/Game/Slots/BP_CodeConsole_NumberWheel.Value` _array_element_2)))
    (switch `int` _output_get
      (:`0`
        (`KismetArrayLibrary.Array_Add` (`self.Suits`) "NewEnumerator0")
        (`KismetSystemLibrary.PrintString` "Club"))
      (:`1`
        (`KismetArrayLibrary.Array_Add` (`self.Suits`) "NewEnumerator1" :!label _label)
        (`KismetSystemLibrary.PrintString` "Heart"))
      (:`2`
        (`KismetArrayLibrary.Array_Add` (`self.Suits`) "NewEnumerator2" :!label _label_2)
        (`KismetSystemLibrary.PrintString` "Spade"))
      (:`3`
        (`KismetArrayLibrary.Array_Add` (`self.Suits`) "NewEnumerator3" :!label _label_3)
        (`KismetSystemLibrary.PrintString` "Diamond"))
      (:`4`
        (goto _label_2))
      (:`5`
        (goto _label))
      (:`6`
        (goto _label_2))
      (:`7`
        (goto _label_3))
      (:`8`
        (goto _label_2))
      (:`9`
        (goto _label_3))))
  (bind (_clubs _hearts _spades _diamonds) (`self.Count`))
  (`|ExecutionSequence`
    (:`then_0`
      (if (== _clubs 4)
        (set `/Game/Slots/W_Slots.Money` (+ (`/Game/Slots/W_Slots.Money` _widget_5) 1000) _widget_5)
        (elif (== _hearts 4)
          (set `/Game/Slots/W_Slots.Money` (+ (`/Game/Slots/W_Slots.Money` _widget_6) 750) _widget_6)
          (elif (== _spades 4)
            (set `/Game/Slots/W_Slots.Money` (+ (`/Game/Slots/W_Slots.Money` _widget_7) 500) _widget_7)
            (elif (== _diamonds 4)
              (set `/Game/Slots/W_Slots.Money` (+ (`/Game/Slots/W_Slots.Money` _widget_8) 250) _widget_8))))))
    (:`then_1`
      (if (== _clubs 3)
        (set `/Game/Slots/W_Slots.Money` (+ (`/Game/Slots/W_Slots.Money` _widget_9) 100) _widget_9)
        (elif (== _hearts 3)
          (set `/Game/Slots/W_Slots.Money` (+ (`/Game/Slots/W_Slots.Money` _widget_10) 75) _widget_10)
          (elif (== _spades 3)
            (set `/Game/Slots/W_Slots.Money` (+ (`/Game/Slots/W_Slots.Money` _widget_11) 50) _widget_11)
            (elif (== _diamonds 3)
              (set `/Game/Slots/W_Slots.Money` (+ (`/Game/Slots/W_Slots.Money` _widget_12) 25) _widget_12))))))
    (:`then_2`
      (if (== _clubs 2)
        (set `/Game/Slots/W_Slots.Money` (+ (`/Game/Slots/W_Slots.Money` _widget_3) 2) _widget_3)))
    (:`then_3`
      (if (== _hearts 2)
        (set `/Game/Slots/W_Slots.Money` (+ (`/Game/Slots/W_Slots.Money` _widget_4) 2) _widget_4)))
    (:`then_4`
      (if (== _spades 2)
        (set `/Game/Slots/W_Slots.Money` (+ (`/Game/Slots/W_Slots.Money` _widget_2) 2) _widget_2)))
    (:`then_5`
      (if (== _diamonds 2)
        (set `/Game/Slots/W_Slots.Money` (+ (`/Game/Slots/W_Slots.Money` _widget) 2) _widget)))))

(fn `Count`
  (returns (Clubs :type Integer) (Hearts :type Integer) (Spades :type Integer) (Diamonds :type Integer))
  (locals (Local_Clubs :type Integer :default 0) (Local_Hearts :type Integer :default 0) (Local_Spades :type Integer :default 0) (Local_Diamonds :type Integer :default 0))
  (set `local.Local_Clubs` 0)
  (set `local.Local_Hearts` 0)
  (set `local.Local_Spades` 0)
  (set `local.Local_Diamonds` 0)
  (for _array_element (`self.Suits`)
    (switch `/Game/Slots/E_Suits` _array_element
      (:`NewEnumerator0`
        (`/Engine/EditorBlueprintResources/StandardMacros.IncrementInt` (`local.Local_Clubs`)))
      (:`NewEnumerator1`
        (`/Engine/EditorBlueprintResources/StandardMacros.IncrementInt` (`local.Local_Hearts`)))
      (:`NewEnumerator2`
        (`/Engine/EditorBlueprintResources/StandardMacros.IncrementInt` (`local.Local_Spades`)))
      (:`NewEnumerator3`
        (`/Engine/EditorBlueprintResources/StandardMacros.IncrementInt` (`local.Local_Diamonds`)))))
  (return (`local.Local_Clubs`) (`local.Local_Hearts`) (`local.Local_Spades`) (`local.Local_Diamonds`)))

(fn `UserConstructionScript`)