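; Builds and shuffles a standard 52-card deck for the casino card assets when play begins.
; BeginPlay runs nested Sequence nodes, one per suit, that set the value string and face texture on the NewCard struct for each rank.
; Each suit's set-member nodes share one Add node that appends to the Deck array, which is shuffled as the final step.
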(event `self.ReceiveBeginPlay`
  (`|ExecutionSequence`
    (:`then_0`
      (`|ExecutionSequence`
        (:`then_0`
          (bind _structout (setmembers `/Game/CasinoAssets/Struc_Deck` :`StructRef` (`self.New Card`) :`Value` "A" :`Texture` "/Game/CasinoAssets/BlackJack/Cards/cardClubsA.cardClubsA")))
        (:`then_1`
          (setmembers `/Game/CasinoAssets/Struc_Deck` :`StructRef` (`self.New Card`) :`Value` "2" :`Texture` "/Game/CasinoAssets/BlackJack/Cards/cardClubs2.cardClubs2"))
        (:`then_2`
          (setmembers `/Game/CasinoAssets/Struc_Deck` :`StructRef` (`self.New Card`) :`Value` "3" :`Texture` "/Game/CasinoAssets/BlackJack/Cards/cardClubs3.cardClubs3"))
        (:`then_3`
          (setmembers `/Game/CasinoAssets/Struc_Deck` :`StructRef` (`self.New Card`) :`Value` "4" :`Texture` "/Game/CasinoAssets/BlackJack/Cards/cardClubs4.cardClubs4"))
        (:`then_4`
          (setmembers `/Game/CasinoAssets/Struc_Deck` :`StructRef` (`self.New Card`) :`Value` "5" :`Texture` "/Game/CasinoAssets/BlackJack/Cards/cardClubs5.cardClubs5"))
        (:`then_5`
          (setmembers `/Game/CasinoAssets/Struc_Deck` :`StructRef` (`self.New Card`) :`Value` "6" :`Texture` "/Game/CasinoAssets/BlackJack/Cards/cardClubs6.cardClubs6"))
        (:`then_6`
          (setmembers `/Game/CasinoAssets/Struc_Deck` :`StructRef` (`self.New Card`) :`Value` "7" :`Texture` "/Game/CasinoAssets/BlackJack/Cards/cardClubs7.cardClubs7"))
        (:`then_7`
          (setmembers `/Game/CasinoAssets/Struc_Deck` :`StructRef` (`self.New Card`) :`Value` "8" :`Texture` "/Game/CasinoAssets/BlackJack/Cards/cardClubs8.cardClubs8"))
        (:`then_8`
          (setmembers `/Game/CasinoAssets/Struc_Deck` :`StructRef` (`self.New Card`) :`Value` "9" :`Texture` "/Game/CasinoAssets/BlackJack/Cards/cardClubs9.cardClubs9"))
        (:`then_9`
          (setmembers `/Game/CasinoAssets/Struc_Deck` :`StructRef` (`self.New Card`) :`Value` "10" :`Texture` "/Game/CasinoAssets/BlackJack/Cards/cardClubs10.cardClubs10"))
        (:`then_10`
          (setmembers `/Game/CasinoAssets/Struc_Deck` :`StructRef` (`self.New Card`) :`Value` "J" :`Texture` "/Game/CasinoAssets/BlackJack/Cards/cardClubsJ.cardClubsJ"))
        (:`then_11`
          (setmembers `/Game/CasinoAssets/Struc_Deck` :`StructRef` (`self.New Card`) :`Value` "Q" :`Texture` "/Game/CasinoAssets/BlackJack/Cards/cardClubsQ.cardClubsQ"))
        (:`then_12`
          (setmembers `/Game/CasinoAssets/Struc_Deck` :`StructRef` (`self.New Card`) :`Value` "K" :`Texture` "/Game/CasinoAssets/BlackJack/Cards/cardClubsK.cardClubsK")))
      (`KismetArrayLibrary.Array_Add` (`self.Deck`) _structout))
    (:`then_1`
      (`|ExecutionSequence`
        (:`then_0`
          (bind _structout_2 (setmembers `/Game/CasinoAssets/Struc_Deck` :`StructRef` (`self.New Card`) :`Value` "A" :`Texture` "/Game/CasinoAssets/BlackJack/Cards/cardDiamondsA.cardDiamondsA")))
        (:`then_1`
          (setmembers `/Game/CasinoAssets/Struc_Deck` :`StructRef` (`self.New Card`) :`Value` "2" :`Texture` "/Game/CasinoAssets/BlackJack/Cards/cardDiamonds2.cardDiamonds2"))
        (:`then_2`
          (setmembers `/Game/CasinoAssets/Struc_Deck` :`StructRef` (`self.New Card`) :`Value` "3" :`Texture` "/Game/CasinoAssets/BlackJack/Cards/cardDiamonds3.cardDiamonds3"))
        (:`then_3`
          (setmembers `/Game/CasinoAssets/Struc_Deck` :`StructRef` (`self.New Card`) :`Value` "4" :`Texture` "/Game/CasinoAssets/BlackJack/Cards/cardDiamonds4.cardDiamonds4"))
        (:`then_4`
          (setmembers `/Game/CasinoAssets/Struc_Deck` :`StructRef` (`self.New Card`) :`Value` "5" :`Texture` "/Game/CasinoAssets/BlackJack/Cards/cardDiamonds5.cardDiamonds5"))
        (:`then_5`
          (setmembers `/Game/CasinoAssets/Struc_Deck` :`StructRef` (`self.New Card`) :`Value` "6" :`Texture` "/Game/CasinoAssets/BlackJack/Cards/cardDiamonds6.cardDiamonds6"))
        (:`then_6`
          (setmembers `/Game/CasinoAssets/Struc_Deck` :`StructRef` (`self.New Card`) :`Value` "7" :`Texture` "/Game/CasinoAssets/BlackJack/Cards/cardDiamonds7.cardDiamonds7"))
        (:`then_7`
          (setmembers `/Game/CasinoAssets/Struc_Deck` :`StructRef` (`self.New Card`) :`Value` "8" :`Texture` "/Game/CasinoAssets/BlackJack/Cards/cardDiamonds8.cardDiamonds8"))
        (:`then_8`
          (setmembers `/Game/CasinoAssets/Struc_Deck` :`StructRef` (`self.New Card`) :`Value` "9" :`Texture` "/Game/CasinoAssets/BlackJack/Cards/cardDiamonds9.cardDiamonds9"))
        (:`then_9`
          (setmembers `/Game/CasinoAssets/Struc_Deck` :`StructRef` (`self.New Card`) :`Value` "10" :`Texture` "/Game/CasinoAssets/BlackJack/Cards/cardDiamonds10.cardDiamonds10"))
        (:`then_10`
          (setmembers `/Game/CasinoAssets/Struc_Deck` :`StructRef` (`self.New Card`) :`Value` "J" :`Texture` "/Game/CasinoAssets/BlackJack/Cards/cardDiamondsJ.cardDiamondsJ"))
        (:`then_11`
          (setmembers `/Game/CasinoAssets/Struc_Deck` :`StructRef` (`self.New Card`) :`Value` "Q" :`Texture` "/Game/CasinoAssets/BlackJack/Cards/cardDiamondsQ.cardDiamondsQ"))
        (:`then_12`
          (setmembers `/Game/CasinoAssets/Struc_Deck` :`StructRef` (`self.New Card`) :`Value` "K" :`Texture` "/Game/CasinoAssets/BlackJack/Cards/cardDiamondsK.cardDiamondsK")))
      (`KismetArrayLibrary.Array_Add` (`self.Deck`) _structout_2))
    (:`then_2`
      (`|ExecutionSequence`
        (:`then_0`
          (bind _structout_3 (setmembers `/Game/CasinoAssets/Struc_Deck` :`StructRef` (`self.New Card`) :`Value` "A" :`Texture` "/Game/CasinoAssets/BlackJack/Cards/cardHeartsA.cardHeartsA")))
        (:`then_1`
          (setmembers `/Game/CasinoAssets/Struc_Deck` :`StructRef` (`self.New Card`) :`Value` "2" :`Texture` "/Game/CasinoAssets/BlackJack/Cards/cardHearts2.cardHearts2"))
        (:`then_2`
          (setmembers `/Game/CasinoAssets/Struc_Deck` :`StructRef` (`self.New Card`) :`Value` "3" :`Texture` "/Game/CasinoAssets/BlackJack/Cards/cardHearts3.cardHearts3"))
        (:`then_3`
          (setmembers `/Game/CasinoAssets/Struc_Deck` :`StructRef` (`self.New Card`) :`Value` "4" :`Texture` "/Game/CasinoAssets/BlackJack/Cards/cardHearts4.cardHearts4"))
        (:`then_4`
          (setmembers `/Game/CasinoAssets/Struc_Deck` :`StructRef` (`self.New Card`) :`Value` "5" :`Texture` "/Game/CasinoAssets/BlackJack/Cards/cardHearts5.cardHearts5"))
        (:`then_5`
          (setmembers `/Game/CasinoAssets/Struc_Deck` :`StructRef` (`self.New Card`) :`Value` "6" :`Texture` "/Game/CasinoAssets/BlackJack/Cards/cardHearts6.cardHearts6"))
        (:`then_6`
          (setmembers `/Game/CasinoAssets/Struc_Deck` :`StructRef` (`self.New Card`) :`Value` "7" :`Texture` "/Game/CasinoAssets/BlackJack/Cards/cardHearts7.cardHearts7"))
        (:`then_7`
          (setmembers `/Game/CasinoAssets/Struc_Deck` :`StructRef` (`self.New Card`) :`Value` "8" :`Texture` "/Game/CasinoAssets/BlackJack/Cards/cardHearts8.cardHearts8"))
        (:`then_8`
          (setmembers `/Game/CasinoAssets/Struc_Deck` :`StructRef` (`self.New Card`) :`Value` "9" :`Texture` "/Game/CasinoAssets/BlackJack/Cards/cardHearts9.cardHearts9"))
        (:`then_9`
          (setmembers `/Game/CasinoAssets/Struc_Deck` :`StructRef` (`self.New Card`) :`Value` "10" :`Texture` "/Game/CasinoAssets/BlackJack/Cards/cardHearts10.cardHearts10"))
        (:`then_10`
          (setmembers `/Game/CasinoAssets/Struc_Deck` :`StructRef` (`self.New Card`) :`Value` "J" :`Texture` "/Game/CasinoAssets/BlackJack/Cards/cardHeartsJ.cardHeartsJ"))
        (:`then_11`
          (setmembers `/Game/CasinoAssets/Struc_Deck` :`StructRef` (`self.New Card`) :`Value` "Q" :`Texture` "/Game/CasinoAssets/BlackJack/Cards/cardHeartsQ.cardHeartsQ"))
        (:`then_12`
          (setmembers `/Game/CasinoAssets/Struc_Deck` :`StructRef` (`self.New Card`) :`Value` "K" :`Texture` "/Game/CasinoAssets/BlackJack/Cards/cardHeartsK.cardHeartsK")))
      (`KismetArrayLibrary.Array_Add` (`self.Deck`) _structout_3))
    (:`then_3`
      (`|ExecutionSequence`
        (:`then_0`
          (bind _structout_4 (setmembers `/Game/CasinoAssets/Struc_Deck` :`StructRef` (`self.New Card`) :`Value` "A" :`Texture` "/Game/CasinoAssets/BlackJack/Cards/cardSpadesA.cardSpadesA")))
        (:`then_1`
          (setmembers `/Game/CasinoAssets/Struc_Deck` :`StructRef` (`self.New Card`) :`Value` "2" :`Texture` "/Game/CasinoAssets/BlackJack/Cards/cardSpades2.cardSpades2"))
        (:`then_2`
          (setmembers `/Game/CasinoAssets/Struc_Deck` :`StructRef` (`self.New Card`) :`Value` "3" :`Texture` "/Game/CasinoAssets/BlackJack/Cards/cardSpades3.cardSpades3"))
        (:`then_3`
          (setmembers `/Game/CasinoAssets/Struc_Deck` :`StructRef` (`self.New Card`) :`Value` "4" :`Texture` "/Game/CasinoAssets/BlackJack/Cards/cardSpades4.cardSpades4"))
        (:`then_4`
          (setmembers `/Game/CasinoAssets/Struc_Deck` :`StructRef` (`self.New Card`) :`Value` "5" :`Texture` "/Game/CasinoAssets/BlackJack/Cards/cardSpades5.cardSpades5"))
        (:`then_5`
          (setmembers `/Game/CasinoAssets/Struc_Deck` :`StructRef` (`self.New Card`) :`Value` "6" :`Texture` "/Game/CasinoAssets/BlackJack/Cards/cardSpades6.cardSpades6"))
        (:`then_6`
          (setmembers `/Game/CasinoAssets/Struc_Deck` :`StructRef` (`self.New Card`) :`Value` "7" :`Texture` "/Game/CasinoAssets/BlackJack/Cards/cardSpades7.cardSpades7"))
        (:`then_7`
          (setmembers `/Game/CasinoAssets/Struc_Deck` :`StructRef` (`self.New Card`) :`Value` "8" :`Texture` "/Game/CasinoAssets/BlackJack/Cards/cardSpades8.cardSpades8"))
        (:`then_8`
          (setmembers `/Game/CasinoAssets/Struc_Deck` :`StructRef` (`self.New Card`) :`Value` "9" :`Texture` "/Game/CasinoAssets/BlackJack/Cards/cardSpades9.cardSpades9"))
        (:`then_9`
          (setmembers `/Game/CasinoAssets/Struc_Deck` :`StructRef` (`self.New Card`) :`Value` "10" :`Texture` "/Game/CasinoAssets/BlackJack/Cards/cardSpades10.cardSpades10"))
        (:`then_10`
          (setmembers `/Game/CasinoAssets/Struc_Deck` :`StructRef` (`self.New Card`) :`Value` "J" :`Texture` "/Game/CasinoAssets/BlackJack/Cards/cardSpadesJ.cardSpadesJ"))
        (:`then_11`
          (setmembers `/Game/CasinoAssets/Struc_Deck` :`StructRef` (`self.New Card`) :`Value` "Q" :`Texture` "/Game/CasinoAssets/BlackJack/Cards/cardSpadesQ.cardSpadesQ"))
        (:`then_12`
          (setmembers `/Game/CasinoAssets/Struc_Deck` :`StructRef` (`self.New Card`) :`Value` "K" :`Texture` "/Game/CasinoAssets/BlackJack/Cards/cardSpadesK.cardSpadesK")))
      (`KismetArrayLibrary.Array_Add` (`self.Deck`) _structout_4))
    (:`then_4`
      (`KismetArrayLibrary.Array_Shuffle` (`self.Deck`)))))

(fn `UserConstructionScript`)